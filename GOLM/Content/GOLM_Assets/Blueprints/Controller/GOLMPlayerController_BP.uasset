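; Player controller that maps keyboard and mouse input to movement, weapon fire, camera, minimap and menu actions for the player's character.
; Hard-coded key events forward to functions defined outside this graph, with held inputs passing true on press and false on release.
; Escape, M and F toggle settings, equipment menu and arc fire from state flags, while Space sets a camera-move flag.
; LeftShift only calls BoostPlayer(false); other boost calls are unwired.
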(event Input|KeyboardEvents|N
  (params (Key :type Key%20Structure :default "AnyKey"))
  (:Pressed
    (Class|GOLMPlayerController|ZoomMiniMap 1e+03)))

(event Input|MouseEvents|LeftMouseButton
  (params (Key :type Key%20Structure :default "AnyKey"))
  (:Pressed
    (Class|GOLMPlayerController|FireHandWeapon true))
  (:Released
    (Class|GOLMPlayerController|FireHandWeapon false)))

(event Input|KeyboardEvents|F
  (params (Key :type Key%20Structure :default "AnyKey"))
  (:Pressed
    (if (Variables|Default|GetbIsArcFireOn)
      (Class|GOLMPlayerController|SetArcFire false)
      (else
        (Class|GOLMPlayerController|SetArcFire true)))))

(event Input|KeyboardEvents|W
  (params (Key :type Key%20Structure :default "AnyKey"))
  (:Pressed
    (Class|GOLMPlayerController|MovePlayerUp true))
  (:Released
    (Class|GOLMPlayerController|MovePlayerUp false)))

(event Input|KeyboardEvents|S
  (params (Key :type Key%20Structure :default "AnyKey"))
  (:Pressed
    (Class|GOLMPlayerController|MovePlayerDown true))
  (:Released
    (Class|GOLMPlayerController|MovePlayerDown false)))

(event Input|KeyboardEvents|A
  (params (Key :type Key%20Structure :default "AnyKey"))
  (:Pressed
    (Class|GOLMPlayerController|MovePlayerLeft true))
  (:Released
    (Class|GOLMPlayerController|MovePlayerLeft false)))

(event Input|KeyboardEvents|D
  (params (Key :type Key%20Structure :default "AnyKey"))
  (:Pressed
    (Class|GOLMPlayerController|MovePlayerRight true))
  (:Released
    (Class|GOLMPlayerController|MovePlayerRight false)))

(event Input|MouseEvents|MouseWheelDown
  (params (Key :type Key%20Structure :default "AnyKey"))
  (:Pressed
    (Class|GOLMPlayerController|ZoomPlayerCamera 4e+02)))

(event Input|KeyboardEvents|K
  (params (Key :type Key%20Structure :default "AnyKey"))
  (:Pressed
    (Class|GOLMPlayerController|KillCharacter)))

(event Input|MouseEvents|MouseWheelUp
  (params (Key :type Key%20Structure :default "AnyKey"))
  (:Pressed
    (Class|GOLMPlayerController|ZoomPlayerCamera -4e+02)))

(event Input|KeyboardEvents|SpaceBar
  (params (Key :type Key%20Structure :default "AnyKey"))
  (:Pressed
    (Variables|Default|SetbMovePlayerCamera true))
  (:Released
    (Variables|Default|SetbMovePlayerCamera false)))

(event Input|KeyboardEvents|Escape
  (params (Key :type Key%20Structure :default "AnyKey"))
  (:Pressed
    (if (Variables|Default|GetbIsInSettingsMenu)
      (Class|GOLMPlayerController|HideinGameSettingsMenu)
      (else
        (Class|GOLMPlayerController|ShowinGameSettingsMenu)))))

(event Input|KeyboardEvents|B
  (params (Key :type Key%20Structure :default "AnyKey"))
  (:Pressed
    (Class|GOLMPlayerController|ZoomMiniMap -1e+03)))

(event Input|KeyboardEvents|M
  (params (Key :type Key%20Structure :default "AnyKey"))
  (:Pressed
    (if (Variables|Default|GetbIsInEquipmentMenu)
      (Class|GOLMPlayerController|HideEquipmentMenu)
      (else
        (Class|GOLMPlayerController|ShowEquipmentMenu)))))

(event Input|KeyboardEvents|LeftShift
  (params (Key :type Key%20Structure :default "AnyKey"))
  (:Pressed
    (Class|GOLMPlayerController|BoostPlayer false)))

(event Input|MouseEvents|RightMouseButton
  (params (Key :type Key%20Structure :default "AnyKey"))
  (:Pressed
    (Class|GOLMPlayerController|RotatePlayerCamera true))
  (:Released
    (Class|GOLMPlayerController|RotatePlayerCamera false)))

(event Input|KeyboardEvents|LeftShift
  (params (Key :type Key%20Structure :default "AnyKey")))

(event Input|KeyboardEvents|E
  (params (Key :type Key%20Structure :default "AnyKey"))
  (:Pressed
    (Class|GOLMPlayerController|FireRightShoulderWeapon true))
  (:Released
    (Class|GOLMPlayerController|FireRightShoulderWeapon false)))

(event Input|KeyboardEvents|Q
  (params (Key :type Key%20Structure :default "AnyKey"))
  (:Pressed
    (Class|GOLMPlayerController|FireLeftShoulderWeapon true))
  (:Released
    (Class|GOLMPlayerController|FireLeftShoulderWeapon false)))

(event Input|KeyboardEvents|H
  (params (Key :type Key%20Structure :default "AnyKey"))
  (:Pressed
    (Class|GOLMPlayerController|GotoLockerRoom)))

(fn ConstructionScript)